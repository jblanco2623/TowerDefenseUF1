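; Enemy actor that travels along a spline path and destroys itself at the end.
; On BeginPlay it casts and stores the CGM game mode, then starts a timeline at a play rate scaled by EnemySpeed.
; The timeline track maps to distance along the referenced spline, setting the actor's location each update, so travel time is independent of path length.
; When the timeline finishes, it prints a debug string before destruction.
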(event `self.ReceiveBeginPlay`
  (bind _spline (`/Game/Splines/SplineLv1.Spline` (`self.Spline`)))
  (bind _ascgm (cast `/Game/Gamemode/CGM` (`GameplayStatics.GetGameMode`)))
  (bind _output_get (set `self.As GMBBP` _ascgm))
  (`/Engine/EditorBlueprintResources/StandardMacros.IsValid` _output_get
    (:`Is Valid`
      (`TimelineComponent.SetPlayRate` (`self.MoveTL`) (/ (`self.EnemySpeed`) 100.0))
      (bind (_direction _movetrack) (`Timeline|MoveTL`)
        (:`Update`
          (`self.K2_SetActorTransform` (`KismetMathLibrary.MakeTransform` (`SplineComponent.GetLocationAtDistanceAlongSpline` _spline (`KismetMathLibrary.Lerp` 0.0 (`SplineComponent.GetSplineLength` _spline) _movetrack) "World"))))
        (:`Finished`
          (`KismetSystemLibrary.PrintString` "Hello")
          (`self.K2_DestroyActor`))))))

(fn `UserConstructionScript`)